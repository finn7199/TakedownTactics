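; Base AI controller for minions that uses sight perception to pick a hero to chase.
; On possession it caches the minion pawn.
; Sighting a hero other than TargetPlayer, while switching is allowed, passes that hero to the minion, starts its move and locks switching.
; Sight updates on TargetPlayer lock switching while it is seen and unlock it when lost; TargetPlayer is never assigned here.
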(event OnTargetPerceptionUpdated(AIPerception)
  (params (Actor :type Actor%20Object%20Reference) (Stimulus :type AI%20Stimulus%20Structure))
  (bind _bsuccessfullysensed (Utilities|Struct|BreakAIStimulus Stimulus))
  (bind _ai_minion_base (Variables|Default|GetAI%20Minion%20Base))
  (bind _returnvalue (Class|AIPerceptionSystem|GetSenseClassforStimulus Stimulus))
  (if (== _returnvalue "/Script/AIModule.AISense_Sight")
    (if (!= Actor (Variables|Default|GetTargetPlayer))
      (bind _asbp_hero_base (Utilities|Casting|CastToBP_Hero_Base Actor))
      (if _bsuccessfullysensed
        (if (Variables|Default|GetCanSwitchTargets)
          (Variables|Default|SetCanSwitchTargets false)
          (Default|SetTargetPlayer _ai_minion_base _asbp_hero_base)
          (Default|MovetoPlayer _ai_minion_base)))
      (elif _bsuccessfullysensed
        (Variables|Default|SetCanSwitchTargets false)
        (else
          (Variables|Default|SetCanSwitchTargets true))))))

(event EventPossess
  (params (PossessedPawn :type Pawn%20Object%20Reference))
  (bind _asbp_ai_minion_base (Utilities|Casting|CastToBP_AI_Minion_Base PossessedPawn))
  (Variables|Default|SetAI%20Minion%20Base _asbp_ai_minion_base))

(fn ConstructionScript)