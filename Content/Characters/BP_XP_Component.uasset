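; Hero component that tracks player XP and level, handling level-ups against an XP threshold map capped at level 10.
; Init loads the map and seeds XP and level from the first player controller's profile.
; Adding XP runs on the server or locally controlled hero, can skip several levels at once, and writes back to that profile.
; The local client also refreshes the HUD, saves progress and plays the level-up animation.
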(event Custom|XP_Component_Init
  (CallFunction|SetupXPMap)
  (bind _asbp_hero_base (Utilities|Casting|CastToBP_Hero_Base (Components|GetOwner)))
  (Variables|Default|SetAs%20BP%20Hero%20Base _asbp_hero_base)
  (bind _asbp_shooter_player_controller (Utilities|Casting|CastToBP_Shooter_PlayerController (Game|GetPlayerController 0)))
  (bind _output_get (Variables|Default|SetAs%20BP%20Shooter%20Player%20Controller _asbp_shooter_player_controller))
  (Variables|Default|SetPlayer%20XP (.player_xp (Variables|/Game/Framework/BP_Shooter_PlayerController.BP_Shooter_PlayerController_C|GetS_PlayerProfile _output_get)))
  (Variables|Default|SetPlayer%20Level (.player_level (Variables|/Game/Framework/BP_Shooter_PlayerController.BP_Shooter_PlayerController_C|GetS_PlayerProfile _output_get)))
  (if (Pawn|IsLocalPlayerController (Variables|Default|GetAs%20BP%20Shooter%20Player%20Controller))
    (Default|UpdateXPAmount (Variables|/Game/Framework/BP_Shooter_PlayerController.BP_Shooter_PlayerController_C|GetWB_IngameHUD (Variables|Default|GetAs%20BP%20Shooter%20Player%20Controller)))
    (Default|UpdateXPLevel (Variables|/Game/Framework/BP_Shooter_PlayerController.BP_Shooter_PlayerController_C|GetWB_IngameHUD (Variables|Default|GetAs%20BP%20Shooter%20Player%20Controller)))
    (Default|SaveXPandLevel (Variables|Default|GetAs%20BP%20Shooter%20Player%20Controller))))

(event Custom|Component_AddXP
  (params (XP_Amount :type Integer))
  (bind _as_bp_shooter_player_controller (Variables|Default|GetAs%20BP%20Shooter%20Player%20Controller))
  (bind _as_bp_hero_base (Variables|Default|GetAs%20BP%20Hero%20Base))
  (bind _wb_ingame_hud (Variables|/Game/Characters/BP_Hero_Base.BP_Hero_Base_C|GetWB%20Ingame%20HUD _as_bp_hero_base))
  (if (or (Networking|IsServer) (Pawn|IsLocallyControlled (Variables|Default|GetAs%20BP%20Hero%20Base)))
    (bind _output_get (Variables|Default|SetPlayer%20XP (+ XP_Amount (Variables|Default|GetPlayer%20XP))))
    (bind (_canlevelup _newlevel) (CallFunction|CheckforLevelUp _output_get))
    (if _canlevelup
      (Variables|Default|SetPlayer%20Level _newlevel))
    (CallFunction|UpdatePlayerControllerProfile)
    (if (Pawn|IsLocallyControlled _as_bp_hero_base)
      (Default|UpdateXPAmount _wb_ingame_hud)
      (Default|UpdateXPLevel _wb_ingame_hud)
      (Default|SaveXPandLevel _as_bp_shooter_player_controller)
      (if _canlevelup
        (Default|PlayUIAnimLevelUp (Variables|/Game/Framework/BP_Shooter_PlayerController.BP_Shooter_PlayerController_C|GetWB_IngameHUD _as_bp_shooter_player_controller))))))

(fn SetupXPMap
  (Variables|Default|SetXP%20Map%20Levels (.xp_map_levels (LocalVariables|GetS_XPAndLevels)))
  (return))

(fn CheckforLevelUp
  (params (XP_Amount :type Integer))
  (LocalVariables|SetLocal_CurrentPlayerXP XP_Amount)
  (LocalVariables|SetLocal_CurrentPlayerLvl (Variables|Default|GetPlayer%20Level))
  (if (and (> (LocalVariables|GetLocal_CurrentPlayerXP) (Utilities|Array|Get(acopy) (Variables|Default|GetXP%20Map%20Levels) (LocalVariables|GetLocal_CurrentPlayerLvl))) (< (LocalVariables|GetLocal_CurrentPlayerLvl) 10))
    (LocalVariables|SetLocal_CanLevelUp true)
    (bind _index (Utilities|FlowControl|ForLoopwithBreak (LocalVariables|GetLocal_CurrentPlayerLvl) 10 :!label _label)
      (:LoopBody
        (if (not (> (LocalVariables|GetLocal_CurrentPlayerXP) (Utilities|Array|Get(acopy) (Variables|Default|GetXP%20Map%20Levels) _index)))
          (LocalVariables|SetLocal_CurrentPlayerLvl _index)
          (goto _label Break)))
      (:Completed
        (return (LocalVariables|GetLocal_CanLevelUp) (LocalVariables|GetLocal_CurrentPlayerLvl))))
    (else
      (LocalVariables|SetLocal_CanLevelUp false)
      (return (LocalVariables|GetLocal_CanLevelUp) (LocalVariables|GetLocal_CurrentPlayerLvl)))))

(fn UpdatePlayerControllerProfile
  (Utilities|Struct|SetmembersinS_PlayerProfile (Variables|/Game/Framework/BP_Shooter_PlayerController.BP_Shooter_PlayerController_C|GetS_PlayerProfile (Variables|Default|GetAs%20BP%20Shooter%20Player%20Controller)) (Variables|Default|GetPlayer%20XP) (Variables|Default|GetPlayer%20Level))
  (return))