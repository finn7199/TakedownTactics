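; Shooter game mode that runs an endless-wave match for solo or multiplayer, configured from travel URL options.
; It waits for expected players, spawns each hero from their saved profile (read from PlayerState under seamless travel, otherwise PlayerController), then starts a countdown.
; Waves spawn growing numbers of tougher minions at tagged points, polling until all die before intermission.
; When all players are dead, game over returns to menu or lobby.
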(event Custom|LevelStart_EndlessWave
  ;[1 1 1] Start level
  (Utilities|FlowControl|Delay 0.2)
  (for _array_element (Variables|Default|GetAll_ConnectedControllers)
    (Default|GamestartCountdown _array_element))
  (Utilities|FlowControl|Delay 3.0)
  (for _array_element_2 (Variables|Default|GetAll_ConnectedControllers)
    (Default|EnableAllInput _array_element_2))
  (bind _outactors (Actor|GetAllActorsOfClasswithTag "/Game/Gameplay/BP_SpawnPoint_AI.BP_SpawnPoint_AI_C" "EndlessWave"))
  (Variables|Default|SetAll_SpawnPoints _outactors)
  (Variables|Default|SetGM_EW_WaveNumber 0)
  (Variables|Default|SetGM_EW_EnemyHealthThisWave 1e+02)
  (CallFunction|StartWave))

(event Custom|StartWave
  (Math|Integer|IncrementInt (Variables|Default|GetGM_EW_WaveNumber)
    (:%20%20
      (for _array_element (Variables|Default|GetAll_ConnectedControllers)
        (Default|ClientHUDStartNewWave _array_element (Variables|Default|GetGM_EW_WaveNumber)))
      (bind _spawncount (CallFunction|GMEWGetEnemyCount (Variables|Default|GetGM_EW_WaveNumber) (Utilities|Array|Length (Variables|Default|GetAll_ConnectedControllers))))
      (Variables|Default|SetGM_EW_NoOfEnemiesThisWave _spawncount)
      (bind _enemyhealth (CallFunction|GMEWGetEnemyHealth (Variables|Default|GetGM_EW_WaveNumber)))
      (Variables|Default|SetGM_EW_EnemyHealthThisWave _enemyhealth)
      (CallFunction|WaveSpawning))))

(event Custom|RespawnAfterDying
  (params (PlayerController :type BP%20Shooter%20Player%20Controller%20Object%20Reference))
  (Pawn|UnPossess PlayerController)
  (bind _newpawn (CallFunction|RespawnPawnforController PlayerController (Class|GameModeBase|FindPlayerStart PlayerController (Utilities|String|ToString(Integer) (Utilities|Array|FindItem (Variables|Default|GetAll_ConnectedControllers) PlayerController)))))
  (Pawn|Possess PlayerController _newpawn))

(event Custom|WaveSpawning
  (Variables|Default|SetGM_EW_SpawnCount 0)
  (bind _returnvalue (Game|SpawnActorfromClass "/Game/AI/BP_AI_Minion_Base.BP_AI_Minion_Base_C" (Transformation|GetActorTransform (.OutItem (Utilities|Array|Random (Variables|Default|GetAll_SpawnPoints)))) "Undefined" "MultiplyWithRoot" 0 0 :!label _label))
  (Utilities|IsValid _returnvalue
    (:Is%20Valid
      (Math|Integer|IncrementInt (Variables|Default|GetGM_EW_SpawnCount)
        (:%20%20
          (CallFunction|GMEWSetupEnemy _returnvalue)
          (if (== (Variables|Default|GetGM_EW_SpawnCount) (Variables|Default|GetGM_EW_NoOfEnemiesThisWave))
            (Variables|Default|SetGM_EW_WaitForWaveEnd false :!label _label_2)
            (bind _outactors (Actor|GetAllActorsOfClass "/Game/AI/BP_AI_Minion_Base.BP_AI_Minion_Base_C"))
            (bind _array_element (Utilities|Array|ForEachLoopwithBreak _outactors :!label _label_3)
              (:LoopBody
                (if (Variables|/Game/AI/BP_AI_Minion_Base.BP_AI_Minion_Base_C|GetIsAlive _array_element)
                  (Variables|Default|SetGM_EW_WaitForWaveEnd true)
                  (goto _label_3 Break)))
              (:Completed
                (if (Variables|Default|GetGM_EW_WaitForWaveEnd)
                  (Utilities|FlowControl|Delay 0.5)
                  (goto _label_2)
                  (else
                    (CallFunction|WaveIntermission)))))
            (else
              (Utilities|FlowControl|Delay (Math|Conversions|ToFloat(Integer) (/ (Math|Random|RandomIntegerinRange 15 25) 10)))
              (goto _label))))))
    (:Is%20Not%20Valid
      (Utilities|FlowControl|Delay 0.2)
      (goto _label))))

(event Custom|WaveIntermission
  (Development|PrintString "Wave Ended: Intermission ..." true true "(R=0.000000,G=1.000000,B=0.000000,A=1.000000)" 5.0)
  (Utilities|FlowControl|Delay 3.0)
  (Development|PrintString "Intermission Ended: New Wave Starting ..." true true "(R=0.000000,G=1.000000,B=0.000000,A=1.000000)" 5.0)
  (CallFunction|StartWave))

(event Custom|GM_EW_GameOver
  (for _array_element (Variables|Default|GetAll_ConnectedControllers)
    (Default|ShowGameOverScreen _array_element (- (Variables|Default|GetGM_EW_WaveNumber) 1)))
  (Utilities|FlowControl|Delay 3.0)
  (if (Variables|Default|GetIsSoloGame)
    (Development|ExecuteConsoleCommand "servertravel MainMenu_Map" (Game|GetPlayerController 0))
    (else
      (Development|ExecuteConsoleCommand "servertravel LobbyMenu_Map" (Game|GetPlayerController 0)))))

(event EventBeginPlay
  ;[1 1 1] Begin play
  (CallFunction|SetGameOptions (Variables|Default|GetOptionsString))
  (Variables|Default|SetIsGameModeReady true))

(event EventHandleStartingNewPlayer
  (params (NewPlayer :type Player%20Controller%20Object%20Reference))
  ;[1 1 1] Handle starting new player
  (bind _asbp_shooter_player_controller (Utilities|Casting|CastToBP_Shooter_PlayerController NewPlayer))
  (Default|LoadProfile _asbp_shooter_player_controller)
  (Utilities|Array|Add (Variables|Default|GetAll_ConnectedControllers) _asbp_shooter_player_controller)
  (if (Variables|Default|GetIsGameModeReady) :!label _label
    (if (Variables|Default|GetIsSoloGame)
      (Class|GameModeBase|RestartPlayeratPlayerStart (Utilities|Array|Get(acopy) (Variables|Default|GetAll_ConnectedControllers)) (Class|GameModeBase|FindPlayerStart 0 "0"))
      (CallFunction|LevelStartEndlessWave)
      (elif (== (Variables|Default|GetNo_ExpectedPlayers) (Utilities|Array|Length (Variables|Default|GetAll_ConnectedControllers)))
        (Utilities|FlowControl|Delay 0.5)
        (for (_array_element _array_index) (Variables|Default|GetAll_ConnectedControllers)
          (Class|GameModeBase|RestartPlayeratPlayerStart _array_element (Class|GameModeBase|FindPlayerStart _array_element (Utilities|String|ToString(Integer) _array_index))))
        (switch Utilities|FlowControl|Switch|SwitchonE_GameModes (Variables|Default|GetGameMode)
          (:NewEnumerator0
            (CallFunction|LevelStartEndlessWave)))))
    (else
      (Utilities|FlowControl|Delay 0.1)
      (goto _label))))

(event EventOnLogout
  (params (ExitingController :type Controller%20Object%20Reference))
  ;[1 1 1] Logout
  (bind _asbp_shooter_player_controller (Utilities|Casting|CastToBP_Shooter_PlayerController ExitingController))
  (Utilities|Array|RemoveItem (Variables|Default|GetAll_ConnectedControllers) _asbp_shooter_player_controller)
  (Math|Integer|DecrementInt (Variables|Default|GetNo_ExpectedPlayers)))

(fn ConstructionScript)

(fn SpawnDefaultPawnfor
  (params (NewPlayer :type Controller%20Object%20Reference) (StartSpot :type Actor%20Object%20Reference))
  (if (Variables|Default|GetSeamless%20Travel%20Enabled)
    (bind _asbp_shooter_playerstate (Utilities|Casting|CastToBP_Shooter_Playerstate (Variables|/Script/Engine.Controller|GetPlayerState NewPlayer)))
    (LocalVariables|SetLocal_CharacterClass (.characterclass (Variables|/Game/Framework/BP_Shooter_Playerstate.BP_Shooter_Playerstate_C|GetS_PlayerProfile _asbp_shooter_playerstate)))
    (LocalVariables|SetLocal_ModelName (.modelname (Variables|/Game/Framework/BP_Shooter_Playerstate.BP_Shooter_Playerstate_C|GetS_PlayerProfile _asbp_shooter_playerstate)))
    (LocalVariables|SetLocal_SkinName (.skinname (Variables|/Game/Framework/BP_Shooter_Playerstate.BP_Shooter_Playerstate_C|GetS_PlayerProfile _asbp_shooter_playerstate)))
    (else
      (bind _asbp_shooter_player_controller (Utilities|Casting|CastToBP_Shooter_PlayerController NewPlayer))
      (LocalVariables|SetLocal_CharacterClass (.CharacterClass (Utilities|Struct|BreakS_PlayerProfile (Variables|/Game/Framework/BP_Shooter_PlayerController.BP_Shooter_PlayerController_C|GetS_PlayerProfile _asbp_shooter_player_controller))))
      (LocalVariables|SetLocal_ModelName (.ModelName (Utilities|Struct|BreakS_PlayerProfile (Variables|/Game/Framework/BP_Shooter_PlayerController.BP_Shooter_PlayerController_C|GetS_PlayerProfile _asbp_shooter_player_controller))))
      (LocalVariables|SetLocal_SkinName (.SkinName (Utilities|Struct|BreakS_PlayerProfile (Variables|/Game/Framework/BP_Shooter_PlayerController.BP_Shooter_PlayerController_C|GetS_PlayerProfile _asbp_shooter_player_controller))))))
  (bind _returnvalue (Game|SpawnActorfromClass (LocalVariables|GetLocal_CharacterClass) (Transformation|GetActorTransform StartSpot) "Undefined" "MultiplyWithRoot" 0 0))
  (bind _asbp_hero_base (Utilities|Casting|CastToBP_Hero_Base _returnvalue))
  (Variables|/Game/Characters/BP_Hero_Base.BP_Hero_Base_C|SetModelName _asbp_hero_base (LocalVariables|GetLocal_ModelName))
  (Variables|/Game/Characters/BP_Hero_Base.BP_Hero_Base_C|SetSkinName _asbp_hero_base (LocalVariables|GetLocal_SkinName))
  (return _asbp_hero_base))

(fn RespawnPawnforController
  (params (PlayerController :type BP%20Shooter%20Player%20Controller%20Object%20Reference) (PlayerStart :type Actor%20Object%20Reference))
  (bind _s_playerprofile (Variables|/Game/Framework/BP_Shooter_PlayerController.BP_Shooter_PlayerController_C|GetS_PlayerProfile PlayerController))
  (bind (_playername _characterrowname _characterclass _modelname _skinname) (Utilities|Struct|BreakS_PlayerProfile _s_playerprofile))
  (if (Variables|Default|GetSeamless%20Travel%20Enabled)
    (bind _asbp_shooter_playerstate (Utilities|Casting|CastToBP_Shooter_Playerstate (Variables|/Script/Engine.Controller|GetPlayerState PlayerController)))
    (LocalVariables|SetLocal_CharacterClass (.characterclass (Variables|/Game/Framework/BP_Shooter_Playerstate.BP_Shooter_Playerstate_C|GetS_PlayerProfile _asbp_shooter_playerstate)))
    (LocalVariables|SetLocal_ModelName (.modelname (Variables|/Game/Framework/BP_Shooter_Playerstate.BP_Shooter_Playerstate_C|GetS_PlayerProfile _asbp_shooter_playerstate)))
    (LocalVariables|SetLocal_SkinName (.skinname (Variables|/Game/Framework/BP_Shooter_Playerstate.BP_Shooter_Playerstate_C|GetS_PlayerProfile _asbp_shooter_playerstate)))
    (else
      (LocalVariables|SetLocal_CharacterClass _characterclass)
      (LocalVariables|SetLocal_ModelName _modelname)
      (LocalVariables|SetLocal_SkinName _skinname)))
  (bind _returnvalue (Game|SpawnActorfromClass (LocalVariables|GetLocal_CharacterClass) (Transformation|GetActorTransform PlayerStart) "Undefined" "MultiplyWithRoot" 0 0))
  (bind _asbp_hero_base (Utilities|Casting|CastToBP_Hero_Base _returnvalue))
  (Variables|/Game/Characters/BP_Hero_Base.BP_Hero_Base_C|SetModelName _asbp_hero_base (LocalVariables|GetLocal_ModelName))
  (Variables|/Game/Characters/BP_Hero_Base.BP_Hero_Base_C|SetSkinName _asbp_hero_base (LocalVariables|GetLocal_SkinName))
  (Variables|/Game/Characters/BP_Hero_Base.BP_Hero_Base_C|SetDeathRespawn _asbp_hero_base true)
  (return _asbp_hero_base))

(fn GMEWGetEnemyCount
  (params (WaveNumber :type Integer) (NoOfPlayers :type Integer))
  (bind _output_get (LocalVariables|SetLocal_NewSpawnCount (+ (+ WaveNumber (* NoOfPlayers 2)) (Variables|Default|GetGM_EW_NoOfEnemiesThisWave))))
  (if (<= _output_get 5)
    (LocalVariables|SetLocal_NewSpawnCount 6))
  (return (LocalVariables|GetLocal_NewSpawnCount)))

(fn GMEWGetEnemyHealth
  (params (WaveNumber :type Integer))
  (if (== WaveNumber 1)
    (LocalVariables|SetLocal_NewHealth 1e+02)
    (else
      (LocalVariables|SetLocal_NewHealth (+ (Variables|Default|GetGM_EW_EnemyHealthThisWave) 1e+01))))
  (return (LocalVariables|GetLocal_NewHealth)))

(fn GMEWSetupEnemy
  (params (Enemy :type BP%20AI%20Minion%20Base%20Object%20Reference))
  (Variables|/Game/AI/BP_AI_Minion_Base.BP_AI_Minion_Base_C|SetHealth Enemy (Variables|Default|GetGM_EW_EnemyHealthThisWave))
  (return))

(fn SetGameOptions
  (params (GameOptionString :type String))
  (switch string (Class|GameplayStatics|ParseOption GameOptionString "GameMode")
    (:EndlessWave
      (Variables|Default|SetGameMode "NewEnumerator0")
      (Variables|Default|SetNo_ExpectedPlayers (Math|Conversions|ToInteger(Byte) (Class|GameplayStatics|ParseOption GameOptionString "NoOfConnectedPlayers")))
      (switch string (Class|GameplayStatics|ParseOption GameOptionString "IsSolo")
        (:True
          (Variables|Default|SetIsSoloGame true))
        (:False
          (Variables|Default|SetIsSoloGame false)))
      (switch string (Class|GameplayStatics|ParseOption GameOptionString "UseSeamlessTravel")
        (:True
          (Variables|Default|SetSeamless%20Travel%20Enabled true)
          (Variables|Default|SetbUseSeamlessTravel true))
        (:False
          (Variables|Default|SetSeamless%20Travel%20Enabled false)
          (Variables|Default|SetbUseSeamlessTravel false)))
      (return))))

(fn GMEWPlayerDied
  (for _array_element (Variables|Default|GetAll_ConnectedControllers)
    (bind _asbp_hero_base (Utilities|Casting|CastToBP_Hero_Base (Pawn|GetControlledPawn _array_element))
      (:then
        _)
      (:CastFailed
        _))
    (if (not (Variables|/Game/Characters/BP_Hero_Base.BP_Hero_Base_C|GetIsAlive _asbp_hero_base))
      (Math|Integer|IncrementInt (LocalVariables|GetLocal_DeadPlayerCount))))
  (if (== (LocalVariables|GetLocal_DeadPlayerCount) (Utilities|Array|Length (Variables|Default|GetAll_ConnectedControllers)))
    (CallFunction|GMEWGameOver))
  (return))