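; Game mode for the multiplayer lobby that tracks connected menu controllers, ready states, selected game mode and player profiles.
; Joins and logouts maintain the player arrays, and a flag-driven UpdateLobby pushes selected changes to every controller and copies profiles into player states.
; Lobby characters spawn on free player spots and take mesh, animation and skins from a customisation data table.
; Committed looks are multicast, while previews use client-only calls.
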(event Custom|UpdateLobby
  (params (PlayerNames :type Boolean) (LevelSelection :type Boolean) (CharacterSelection :type Boolean) (PlayersReady :type Boolean) (GameMode :type Boolean))
  (Utilities|Array|Clear (Variables|Default|GetAll_PlayerProfiles))
  (for (_array_element _array_index) (Variables|Default|GetAll_ConnectedPlayers)
    (Utilities|Array|SetArrayElem (Variables|Default|GetAll_PlayerProfiles) _array_index (Variables|/Game/Framework/BP_MenuController.BP_MenuController_C|GetPlayer%20Profile _array_element) true)
    (bind _asbp_shooter_playerstate (Utilities|Casting|CastToBP_Shooter_Playerstate (Variables|/Script/Engine.Controller|GetPlayerState _array_element)))
    (Variables|/Game/Framework/BP_Shooter_Playerstate.BP_Shooter_Playerstate_C|SetS_PlayerProfile _asbp_shooter_playerstate (Variables|/Game/Framework/BP_MenuController.BP_MenuController_C|GetPlayer%20Profile _array_element)))
  (for (_array_element_2 _array_index_2) (Variables|Default|GetAll_ConnectedPlayers)
    (if PlayerNames
      (Default|UpdatePlayerNames _array_element_2 (Variables|Default|GetAll_PlayerProfiles)))
    (if LevelSelection
      (Default|UpdateLevelSelection _array_element_2 (Variables|Default|GetSelectedLevelName)))
    (if CharacterSelection
      (CallFunction|UpdateSelectedCharacter _array_index_2))
    (if PlayersReady
      (Default|UpdatePlayerReady _array_element_2 (Variables|Default|GetIsPlayerReady)))
    (if GameMode
      (Default|UpdateGameMode _array_element_2 (Variables|Default|GetSelectedGameMode)))))

(event Custom|UpdateSelectedCharacter
  (params (PlayerIndex :type Integer))
  (bind _all_connectedplayers (Variables|Default|GetAll_ConnectedPlayers))
  (bind _all_connectedplayers_2 (Variables|Default|GetAll_ConnectedPlayers))
  (bind _all_playerprofiles (Variables|Default|GetAll_PlayerProfiles))
  (bind _output (Utilities|Array|Get(acopy) _all_connectedplayers PlayerIndex))
  (bind _output_2 (Utilities|Array|Get(acopy) _all_connectedplayers_2 PlayerIndex))
  (bind _output_3 (Utilities|Array|Get(acopy) _all_playerprofiles PlayerIndex))
  (if (== (Variables|/Game/Framework/BP_MenuController.BP_MenuController_C|GetBP_LobbyCharacter _output) 0)
    (bind _availableplayerspot (CallFunction|GetLobbyPlayerSpots))
    (Variables|/Game/Gameplay/Lobby/BP_Lobby_PlayerSpot.BP_Lobby_PlayerSpot_C|SetIsSpotUsed _availableplayerspot true)
    (bind _returnvalue (Game|SpawnActorfromClass "/Game/Gameplay/Lobby/BP_LobbyCharacter.BP_LobbyCharacter_C" (Transformation|GetActorTransform _availableplayerspot) "Undefined" "MultiplyWithRoot" _output 0))
    (Variables|/Game/Framework/BP_MenuController.BP_MenuController_C|SetBP_LobbyCharacter _output_2 _returnvalue)
    (Variables|/Game/Framework/BP_MenuController.BP_MenuController_C|SetBP_LobbyPlayerSpot _output_2 _availableplayerspot))
  (Default|MulticastSetPlayerName (Variables|/Game/Framework/BP_MenuController.BP_MenuController_C|GetBP_LobbyCharacter (Utilities|Array|Get(acopy) (Variables|Default|GetAll_ConnectedPlayers) PlayerIndex)) (.playername _output_3))
  (bind _returnvalue_2 (Utilities|GetDataTableRow "/Game/Characters/CharCustomisation_Table.CharCustomisation_Table" (.characterrowname _output_3))
    (:then
      (Default|MulticastSetCharacterMesh (Variables|/Game/Framework/BP_MenuController.BP_MenuController_C|GetBP_LobbyCharacter (Utilities|Array|Get(acopy) (Variables|Default|GetAll_ConnectedPlayers) PlayerIndex)) (.Model (Utilities|Struct|BreakS_ModelAndSkins (.Value (Utilities|Map|Find (.ModelsAndSkins (Utilities|Struct|BreakS_CharCustomisation _returnvalue_2)) (.modelname _output_3))))))
      (Default|MulticastPlayMeshAnim (Variables|/Game/Framework/BP_MenuController.BP_MenuController_C|GetBP_LobbyCharacter (Utilities|Array|Get(acopy) (Variables|Default|GetAll_ConnectedPlayers) PlayerIndex)) (.LobbyAnimation (Utilities|Struct|BreakS_ModelAndSkins (.Value (Utilities|Map|Find (.ModelsAndSkins (Utilities|Struct|BreakS_CharCustomisation _returnvalue_2)) (.modelname _output_3))))))
      (if (.Use_Skin0 (Utilities|Struct|BreakS_ModelAndSkins (.Value (Utilities|Map|Find (.ModelsAndSkins (Utilities|Struct|BreakS_CharCustomisation _returnvalue_2)) (.modelname _output_3)))))
        (Default|MulticastSetSkinMaterial (Variables|/Game/Framework/BP_MenuController.BP_MenuController_C|GetBP_LobbyCharacter (Utilities|Array|Get(acopy) (Variables|Default|GetAll_ConnectedPlayers) PlayerIndex)) (.Skin0_MaterialSlot (Utilities|Struct|BreakS_ModelAndSkins (.Value (Utilities|Map|Find (.ModelsAndSkins (Utilities|Struct|BreakS_CharCustomisation _returnvalue_2)) (.modelname _output_3))))) (.Value (Utilities|Map|Find (.Skin0_Skins (Utilities|Struct|BreakS_ModelAndSkins (.Value (Utilities|Map|Find (.ModelsAndSkins (Utilities|Struct|BreakS_CharCustomisation _returnvalue_2)) (.modelname _output_3))))) (.skinname _output_3)))))
      (if (.Use_Skin1 (Utilities|Struct|BreakS_ModelAndSkins (.Value (Utilities|Map|Find (.ModelsAndSkins (Utilities|Struct|BreakS_CharCustomisation _returnvalue_2)) (.modelname _output_3)))))
        (Default|MulticastSetSkinMaterial (Variables|/Game/Framework/BP_MenuController.BP_MenuController_C|GetBP_LobbyCharacter (Utilities|Array|Get(acopy) (Variables|Default|GetAll_ConnectedPlayers) PlayerIndex)) (.Skin1_MaterialSlot (Utilities|Struct|BreakS_ModelAndSkins (.Value (Utilities|Map|Find (.ModelsAndSkins (Utilities|Struct|BreakS_CharCustomisation _returnvalue_2)) (.modelname _output_3))))) (.Value (Utilities|Map|Find (.Skin1_Skins (Utilities|Struct|BreakS_ModelAndSkins (.Value (Utilities|Map|Find (.ModelsAndSkins (Utilities|Struct|BreakS_CharCustomisation _returnvalue_2)) (.modelname _output_3))))) (.skinname _output_3))))))))

(event Custom|UpdateCharForController
  (params (Controller :type BP%20Menu%20Controller%20Object%20Reference) (PlayerProfile :type S%20Player%20Profile%20Structure))
  (bind _all_connectedplayers (Variables|Default|GetAll_ConnectedPlayers))
  (bind _returnvalue (Utilities|Array|FindItem _all_connectedplayers Controller))
  (Utilities|Array|SetArrayElem (Variables|Default|GetAll_PlayerProfiles) _returnvalue PlayerProfile true)
  (bind _asbp_shooter_playerstate (Utilities|Casting|CastToBP_Shooter_Playerstate (Variables|/Script/Engine.Controller|GetPlayerState Controller)))
  (Variables|/Game/Framework/BP_Shooter_Playerstate.BP_Shooter_Playerstate_C|SetS_PlayerProfile _asbp_shooter_playerstate PlayerProfile)
  (CallFunction|UpdateSelectedCharacter _returnvalue))

(event Custom|PreviewCharForController
  (params (Controller :type BP%20Menu%20Controller%20Object%20Reference) (CharRowName :type Name) (ModelName :type Name) (SkinName :type Name))
  (bind _bp_lobbycharacter (Variables|/Game/Framework/BP_MenuController.BP_MenuController_C|GetBP_LobbyCharacter Controller))
  (bind _returnvalue (Utilities|GetDataTableRow "/Game/Characters/CharCustomisation_Table.CharCustomisation_Table" CharRowName)
    (:then
      (Default|ClientSetCharacterMesh _bp_lobbycharacter (.Model (Utilities|Struct|BreakS_ModelAndSkins (.Value (Utilities|Map|Find (.ModelsAndSkins (Utilities|Struct|BreakS_CharCustomisation _returnvalue)) ModelName)))))
      (Default|ClientPlayMeshAnim _bp_lobbycharacter (.LobbyAnimation (Utilities|Struct|BreakS_ModelAndSkins (.Value (Utilities|Map|Find (.ModelsAndSkins (Utilities|Struct|BreakS_CharCustomisation _returnvalue)) ModelName)))))
      (if (.Use_Skin0 (Utilities|Struct|BreakS_ModelAndSkins (.Value (Utilities|Map|Find (.ModelsAndSkins (Utilities|Struct|BreakS_CharCustomisation _returnvalue)) ModelName))))
        (Default|ClientSetSkinMaterial _bp_lobbycharacter (.Skin0_MaterialSlot (Utilities|Struct|BreakS_ModelAndSkins (.Value (Utilities|Map|Find (.ModelsAndSkins (Utilities|Struct|BreakS_CharCustomisation _returnvalue)) ModelName)))) (.Value (Utilities|Map|Find (.Skin0_Skins (Utilities|Struct|BreakS_ModelAndSkins (.Value (Utilities|Map|Find (.ModelsAndSkins (Utilities|Struct|BreakS_CharCustomisation _returnvalue)) ModelName)))) SkinName))))
      (if (.Use_Skin1 (Utilities|Struct|BreakS_ModelAndSkins (.Value (Utilities|Map|Find (.ModelsAndSkins (Utilities|Struct|BreakS_CharCustomisation _returnvalue)) ModelName))))
        (Default|ClientSetSkinMaterial _bp_lobbycharacter (.Skin1_MaterialSlot (Utilities|Struct|BreakS_ModelAndSkins (.Value (Utilities|Map|Find (.ModelsAndSkins (Utilities|Struct|BreakS_CharCustomisation _returnvalue)) ModelName)))) (.Value (Utilities|Map|Find (.Skin1_Skins (Utilities|Struct|BreakS_ModelAndSkins (.Value (Utilities|Map|Find (.ModelsAndSkins (Utilities|Struct|BreakS_CharCustomisation _returnvalue)) ModelName)))) SkinName)))))))

(event Custom|SetPlayerReady
  (params (PlayerController :type BP%20Menu%20Controller%20Object%20Reference) (IsReady :type Boolean))
  (Utilities|Array|SetArrayElem (Variables|Default|GetIsPlayerReady) (Utilities|Array|FindItem (Variables|Default|GetAll_ConnectedPlayers) PlayerController) IsReady)
  (CallFunction|UpdateLobby false false false true false))

(event Custom|SetSelectedGameMode
  (params (SelectedGameMode :type E_GameModes%20Enum :default "NewEnumerator0"))
  (Variables|Default|SetSelectedGameMode SelectedGameMode)
  (CallFunction|UpdateLobby false false false false true))

(event EventOnLogout
  (params (ExitingController :type Controller%20Object%20Reference))
  (bind _asbp_menu_controller (Utilities|Casting|CastToBP_MenuController ExitingController))
  (if true
    _
    (else
      (Actor|DestroyActor (Variables|/Game/Framework/BP_MenuController.BP_MenuController_C|GetBP_LobbyCharacter _asbp_menu_controller))
      (Variables|/Game/Gameplay/Lobby/BP_Lobby_PlayerSpot.BP_Lobby_PlayerSpot_C|SetIsSpotUsed (Variables|/Game/Framework/BP_MenuController.BP_MenuController_C|GetBP_LobbyPlayerSpot _asbp_menu_controller) false)))
  (Utilities|Array|RemoveIndex (Variables|Default|GetIsPlayerReady) (Utilities|Array|FindItem (Variables|Default|GetAll_ConnectedPlayers) _asbp_menu_controller))
  (Utilities|Array|RemoveIndex (Variables|Default|GetAll_ConnectedPlayers) (Utilities|Array|FindItem (Variables|Default|GetAll_ConnectedPlayers) _asbp_menu_controller))
  (CallFunction|UpdateLobby true false true true false))

(event EventHandleStartingNewPlayer
  (params (NewPlayer :type Player%20Controller%20Object%20Reference))
  (bind _returnvalue (Game|GetCurrentLevelName true))
  (switch string _returnvalue
    (:LobbyMenu_Map
      (bind _asbp_menu_controller (Utilities|Casting|CastToBP_MenuController NewPlayer))
      (bind _returnvalue_2 (Utilities|Array|Add (Variables|Default|GetAll_ConnectedPlayers) _asbp_menu_controller))
      (Utilities|Array|SetArrayElem (Variables|Default|GetIsPlayerReady) _returnvalue_2 false true)
      (Default|CreateLobbyMenu _asbp_menu_controller)
      (Default|InitialSetup _asbp_menu_controller))))

(fn ConstructionScript)

(fn GetLobbyPlayerSpots
  (if (== (Utilities|Array|Length (Variables|Default|GetAll_Lobby_PlayerSpots)) 0)
    (bind _outactors (Actor|GetAllActorsOfClass "/Game/Gameplay/Lobby/BP_Lobby_PlayerSpot.BP_Lobby_PlayerSpot_C"))
    (Variables|Default|SetAll_Lobby_PlayerSpots _outactors))
  (bind _array_element (Utilities|Array|ForEachLoopwithBreak (Variables|Default|GetAll_Lobby_PlayerSpots) :!label _label)
    (:LoopBody
      (if (not (Variables|/Game/Gameplay/Lobby/BP_Lobby_PlayerSpot.BP_Lobby_PlayerSpot_C|GetIsSpotUsed _array_element))
        (goto _label Break)))
    (:Completed
      (return _array_element))))