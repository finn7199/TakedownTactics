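; Shooter game instance that handles menus, the saved player profile, solo and multiplayer game starts, and pausing.
; The profile persists through an SG_PlayerProfile save slot, loaded or created when the main menu opens.
; Multiplayer hosts or joins LAN-switchable sessions via a listen-server lobby, and both modes pass match settings to maps as URL options.
; Pause truly pauses only in solo, while multiplayer just toggles the pause menu.
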(event Custom|StartSoloGame
  (Variables|Default|SetIsSolo true)
  (CallFunction|MakeOptionsString "NoOfConnectedPlayers" "1")
  (CallFunction|MakeOptionsString "IsSolo" (Utilities|String|ToString(Boolean) (Variables|Default|GetIsSolo)))
  (CallFunction|MakeOptionsString "UseSeamlessTravel" (Utilities|String|ToString(Boolean) (Variables|Default|GetSeamlessTravelEnabled)))
  (CallFunction|MakeOptionsString "GameMode" (Variables|Default|GetSelectedGameMode))
  (Game|OpenLevel(byName) "Map_01" true (Variables|Default|GetOptionsString)))

(event Custom|ChangePlayerName
  (params (PlayerNameText :type Text))
  (Utilities|Struct|SetmembersinS_PlayerProfile (Variables|Default|GetplayerProfileInfo) PlayerNameText)
  (CallFunction|SaveProfile))

(event Custom|CreateMultiplayerSession
  (Variables|Default|SetIsSolo false)
  (|Session (Game|GetPlayerController 0) 4 (Variables|Default|GetisLAN)
    (:OnSuccess
      (Game|OpenLevel(byName) "LobbyMenu_Map" true "listen"))
    (:OnFailure
      (Development|PrintString "Failed to create a multiplayer session"))))

(event Custom|JoinMultiplayerSession
  (params (SessionResult :type Blueprint%20Session%20Result%20Structure))
  (Variables|Default|SetIsSolo false)
  (|JoinSession (Game|GetPlayerController 0) SessionResult
    (:OnFailure
      (Development|PrintString "Failed to join a multiplayer session"))))

(event Custom|TravelToMap
  (params (noOfConnectedPlayers :type Integer) (mapName :type String))
  (CallFunction|MakeOptionsString "NoOfConnectedPlayers" (Utilities|String|ToString(Integer) noOfConnectedPlayers))
  (CallFunction|MakeOptionsString "IsSolo" (Utilities|String|ToString(Boolean) (Variables|Default|GetIsSolo)))
  (CallFunction|MakeOptionsString "UseSeamlessTravel" (Utilities|String|ToString(Boolean) (Variables|Default|GetSeamlessTravelEnabled)))
  (CallFunction|MakeOptionsString "GameMode" (Variables|Default|GetSelectedGameMode))
  (Development|ExecuteConsoleCommand (Utilities|String|Append "servertravel " mapName (Variables|Default|GetOptionsString)) (Game|GetPlayerController 0)))

(event Custom|Reset_XP
  (Variables|Default|SetplayerProfileInfo (Utilities|Struct|MakeS_PlayerProfile (.playername (Variables|Default|GetplayerProfileInfo)) "Quinn_Blue" "/Game/Characters/BP_Hero_Quinn_Blue.BP_Hero_Quinn_Blue_C"))
  (CallFunction|SaveProfile))

(fn UIShowMainMenu
  (bind _returnvalue (Game|GetPlayerController 0))
  (CallFunction|CheckforSavedProfile)
  (Utilities|IsValid (Variables|Default|GetWB_MainMenu)
    (:Is%20Valid
      _)
    (:Is%20Not%20Valid
      (bind _returnvalue_2 (UserInterface|CreateWidget "/Game/Widgets/WB_MainMenu.WB_MainMenu_C" _returnvalue))
      (Variables|Default|SetWB_MainMenu _returnvalue_2)))
  (UserInterface|Viewport|AddtoViewport (Variables|Default|GetWB_MainMenu) 0)
  (Input|SetInputModeUIOnly _returnvalue 0 "DoNotLock" false)
  (Variables|/Script/Engine.PlayerController|SetbShowMouseCursor _returnvalue true)
  (return))

(fn CheckforSavedProfile
  (bind _returnvalue (SaveGame|DoesSaveGameExist (Variables|Default|GetplayerProfileSlot)))
  (if _returnvalue
    (bind _assg_player_profile (CallFunction|LoadProfile))
    (Variables|Default|SetSG_PlayerProfile _assg_player_profile)
    (else
      (CallFunction|SaveProfile)))
  (return))

(fn LoadProfile
  (bind _returnvalue (SaveGame|LoadGamefromSlot (Variables|Default|GetplayerProfileSlot)))
  (bind _assg_player_profile (Utilities|Casting|CastToSG_PlayerProfile _returnvalue))
  (Variables|Default|SetplayerProfileInfo (Variables|/Game/SavedData/SG_PlayerProfile.SG_PlayerProfile_C|GetPlayerProfile _assg_player_profile))
  (return _assg_player_profile))

(fn SaveProfile
  (Utilities|IsValid (Variables|Default|GetSG_PlayerProfile)
    (:Is%20Valid
      _)
    (:Is%20Not%20Valid
      (bind _returnvalue (SaveGame|CreateSaveGameObject "/Game/SavedData/SG_PlayerProfile.SG_PlayerProfile_C"))
      (Variables|Default|SetSG_PlayerProfile _returnvalue)))
  (Variables|/Game/SavedData/SG_PlayerProfile.SG_PlayerProfile_C|SetPlayerProfile (Variables|Default|GetSG_PlayerProfile) (Variables|Default|GetplayerProfileInfo))
  (SaveGame|SaveGametoSlot (Variables|Default|GetSG_PlayerProfile) (Variables|Default|GetplayerProfileSlot))
  (return))

(fn UIShowMultiplayerMenu
  (Utilities|IsValid (Variables|Default|GetWB_MultiplayerMenu)
    (:Is%20Valid
      _)
    (:Is%20Not%20Valid
      (bind _returnvalue (UserInterface|CreateWidget "/Game/Widgets/WB_MultiplayerMenu.WB_MultiplayerMenu_C" (Game|GetPlayerController 0)))
      (Variables|Default|SetWB_MultiplayerMenu _returnvalue)))
  (UserInterface|Viewport|AddtoViewport (Variables|Default|GetWB_MultiplayerMenu) 0)
  (return))

(fn ChangeConnectionType
  (if (Variables|Default|GetisLAN)
    (Variables|Default|SetisLAN false)
    (else
      (Variables|Default|SetisLAN true)))
  (return (Variables|Default|GetisLAN)))

(fn UIShowPauseMenu
  (bind _returnvalue (Game|GetPlayerController 0))
  (Utilities|IsValid (Variables|Default|GetWB_PauseMenu)
    (:Is%20Valid
      _)
    (:Is%20Not%20Valid
      (bind _returnvalue_2 (UserInterface|CreateWidget "/Game/Widgets/WB_PauseMenu.WB_PauseMenu_C" _returnvalue))
      (Variables|Default|SetWB_PauseMenu _returnvalue_2)))
  (UserInterface|Viewport|AddtoViewport (Variables|Default|GetWB_PauseMenu) 0)
  (Input|SetInputModeUIOnly _returnvalue 0 "DoNotLock" false)
  (Variables|/Script/Engine.PlayerController|SetbShowMouseCursor _returnvalue true)
  (return))

(fn TogglePauseGame
  (bind _returnvalue (Game|GetPlayerController 0))
  (if (Variables|Default|GetIsSolo)
    (if (Game|IsGamePaused)
      (bind _returnvalue_2 (Game|SetGamePaused false))
      (LocalVariables|SetLcl_isGamePaused _returnvalue_2)
      (Widget|RemovefromParent (Variables|Default|GetWB_PauseMenu) :!label _label)
      (Input|SetInputModeGameOnly _returnvalue false)
      (Variables|/Script/Engine.PlayerController|SetbShowMouseCursor _returnvalue false)
      (bind _asbp_shooter_player_controller (Utilities|Casting|CastToBP_Shooter_PlayerController _returnvalue))
      (Default|UnhideIngameHUD _asbp_shooter_player_controller)
      (else
        (bind _returnvalue_3 (Game|SetGamePaused true))
        (LocalVariables|SetLcl_isGamePaused _returnvalue_3)
        (CallFunction|UIShowPauseMenu :!label _label_2)))
    (elif (Variables|Default|GetMP_isPauseMenuVisible)
      (Variables|Default|SetMP_isPauseMenuVisible false)
      (goto _label)
      (else
        (Variables|Default|SetMP_isPauseMenuVisible true)
        (LocalVariables|SetLcl_isGamePaused true)
        (goto _label_2))))
  (return (LocalVariables|GetLcl_isGamePaused)))

(fn MakeOptionsString
  (params (New%20Option :type String) (New%20Setting :type String))
  (Variables|Default|SetOptionsString (Utilities|String|Append (Variables|Default|GetOptionsString) "?" New%20Option "=" New%20Setting))
  (return))